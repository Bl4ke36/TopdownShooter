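; BP_Player is a top-down player character that moves with Enhanced Input, jumps and turns toward the mouse cursor hit point.
; The rocket input spawns BP_Bullet after a short delay, drawing on the bullet count in the level's BP_AmmoCounter.
; The attack input only draws a debug line trace.
; Any capsule overlap reduces Life, but Shield is unused and Tick's constant-true branch means IsDead is never set.
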(event `self.ReceiveBeginPlay`
  (bind _returnvalue (`GameplayStatics.GetPlayerController` 0))
  ;[1 0.9881 0 0.5] Start
  (`EnhancedInputSubsystemInterface.AddMappingContext` (pcsubsystem `EnhancedInputLocalPlayerSubsystem` _returnvalue) "/Game/IMC_Player.IMC_Player" 0 (struct))
  (set `PlayerController.bShowMouseCursor` true _returnvalue)
  (bind _returnvalue_2 (`GameplayStatics.GetActorOfClass` "/Game/BP_AmmoCounter.BP_AmmoCounter_C"))
  (set `self.AmmoCounter` _returnvalue_2)
  (set `self.Life` 150.0)
  (set `self.Shield` 100.0))

(event `self.ReceiveTick`
  (params (DeltaSeconds :type "Float (single-precision)"))
  (bind (_returnvalue_roll _returnvalue_pitch _returnvalue_yaw) (`KismetMathLibrary.BreakRotator` (`KismetMathLibrary.FindLookAtRotation` (`self.K2_GetActorLocation`) (`.Location` (`GameplayStatics.BreakHitResult` (`PlayerController.GetHitResultUnderCursorByChannel` (`GameplayStatics.GetPlayerController` 0) "TraceTypeQuery1" true))))))
  ;[0.15 0 0 0.5] Update
  (if true
    (`self.K2_SetActorRotation` (`KismetMathLibrary.MakeRotator` 0.0 0.0 _returnvalue_yaw))
    (if (`self.IsJumping`)
      (set `self.IsJumping` (not (`NavMovementInterface.IsFalling` (`self.CharacterMovement`)))))
    (else
      (set `self.IsDead` true))))

(event `EnhancedInput|/Game/IA_Movement`
  (params (ActionValue :type "Vector2D Structure") (ElapsedSeconds :type "Float (double-precision)") (TriggeredSeconds :type "Float (double-precision)") (InputAction :type "InputAction Object Reference" :default "/Game/IA_Movement.IA_Movement"))
  ;[0 0.8558 0.8906 0.5] Movimiento
  (:`Triggered`
    (if (not (`self.IsDead`))
      (`self.AddMovementInput` (`KismetMathLibrary.Conv_Vector2DToVector` ActionValue)))))

(event `EnhancedInput|/Game/IA_Rocket`
  (params (ActionValue :type Boolean) (ElapsedSeconds :type "Float (double-precision)") (TriggeredSeconds :type "Float (double-precision)") (InputAction :type "InputAction Object Reference" :default "/Game/IA_Rocket.IA_Rocket"))
  ;[0.8646 0.3409 0 0.5] Misil
  (:`Started`
    (if (> (`/Game/BP_AmmoCounter.Bullets` (`self.AmmoCounter`)) 0)
      (set `self.IsShooting` true)
      (`KismetSystemLibrary.Delay` 0.2)
      (`|SpawnActorFromClass` "/Game/BP_Bullet.BP_Bullet_C" (`SceneComponent.K2_GetComponentToWorld` (`self.Scene`)) "Undefined" "MultiplyWithRoot" null null)
      (`/Engine/EditorBlueprintResources/StandardMacros.DecrementInt` (`/Game/BP_AmmoCounter.Bullets` (`self.AmmoCounter`)))))
  (:`Completed`
    (set `self.IsShooting` false)))

(event `EnhancedInput|/Game/IA_Jumping`
  (params (ActionValue :type Boolean) (ElapsedSeconds :type "Float (double-precision)") (TriggeredSeconds :type "Float (double-precision)") (InputAction :type "InputAction Object Reference" :default "/Game/IA_Jumping.IA_Jumping"))
  ;[0 0.8558 0.8906 0.5] Movimiento
  (:`Triggered`
    (`self.Jump`)
    (set `self.IsJumping` true)))

(event `EnhancedInput|/Game/IA_Attacking`
  (params (ActionValue :type Boolean) (ElapsedSeconds :type "Float (double-precision)") (TriggeredSeconds :type "Float (double-precision)") (InputAction :type "InputAction Object Reference" :default "/Game/IA_Attacking.IA_Attacking"))
  (bind _scene (`self.Scene`))
  (bind _returnvalue (`SceneComponent.K2_GetComponentLocation` _scene))
  ;[0 0.8021 0.3535 0.5] Shooting
  (:`Started`
    (`KismetSystemLibrary.LineTraceSingle` :`Start` _returnvalue :`End` (+ _returnvalue (* (`SceneComponent.GetForwardVector` _scene) 1000.0)) :`TraceChannel` "TraceTypeQuery1" :`DrawDebugType` "ForDuration" :`DrawTime` 2.0)))

(event `self.CapsuleComponent.OnComponentBeginOverlap`
  (params (OverlappedComponent :type "PrimitiveComponent Object Reference") (OtherActor :type "Actor Object Reference") (OtherComp :type "PrimitiveComponent Object Reference") (OtherBodyIndex :type Integer) (bFromSweep :type Boolean) (SweepResult :type "HitResult Structure (by ref)"))
  (set `self.Life` (- (`self.Life`) 10.0)))

(fn `UserConstructionScript`)