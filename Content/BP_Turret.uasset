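; BP_Turret is a destructible turret that turns on yaw to face the player and shoots when they come within range.
; Tick updates the aim and, while a BP_Player is inside the Sphere, accumulates delta time to spawn a BP_Bullet at the Scene transform every FIreRate seconds.
; Any BP_Bullet overlapping the mesh is destroyed and removes one Life; Tick destroys the turret once Life runs out.
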(event `self.ReceiveTick`
  (params (DeltaSeconds :type "Float (single-precision)"))
  (bind (_returnvalue_roll _returnvalue_pitch) (`KismetMathLibrary.BreakRotator` (`self.K2_GetActorRotation`)))
  (bind (_returnvalue_roll_2 _returnvalue_pitch_2 _returnvalue_yaw) (`KismetMathLibrary.BreakRotator` (`KismetMathLibrary.FindLookAtRotation` (+ (0.0 0.0 0.0) (0.0 0.0 0.0)) (- (`self.K2_GetActorLocation` (`GameplayStatics.GetPlayerPawn` 0)) (`self.K2_GetActorLocation`)))))
  (if (> (`self.Life`) 0.0)
    (`self.K2_SetActorRotation` (`KismetMathLibrary.MakeRotator` _returnvalue_roll _returnvalue_pitch _returnvalue_yaw))
    (if (`self.Shoot`)
      (set `self.FireTime` (+ DeltaSeconds (`self.FireTime`)))
      (if (>= (`self.FireTime`) (`self.FIreRate`))
        (`|SpawnActorFromClass` "/Game/BP_Bullet.BP_Bullet_C" (`SceneComponent.K2_GetComponentToWorld` (`self.Scene`)) "Undefined" "MultiplyWithRoot" null null)
        (set `self.FireTime` 0.0)))
    (else
      (`self.K2_DestroyActor`))))

(event `self.Sphere.OnComponentBeginOverlap`
  (params (OverlappedComponent :type "PrimitiveComponent Object Reference") (OtherActor :type "Actor Object Reference") (OtherComp :type "PrimitiveComponent Object Reference") (OtherBodyIndex :type Integer) (bFromSweep :type Boolean) (SweepResult :type "HitResult Structure (by ref)"))
  (cast `/Game/BP_Player` OtherActor)
  (set `self.Shoot` true))

(event `self.Sphere.OnComponentEndOverlap`
  (params (OverlappedComponent :type "PrimitiveComponent Object Reference") (OtherActor :type "Actor Object Reference") (OtherComp :type "PrimitiveComponent Object Reference") (OtherBodyIndex :type Integer))
  (cast `/Game/BP_Player` OtherActor)
  (set `self.Shoot` false))

(event `self.StaticMesh.OnComponentBeginOverlap`
  (params (OverlappedComponent :type "PrimitiveComponent Object Reference") (OtherActor :type "Actor Object Reference") (OtherComp :type "PrimitiveComponent Object Reference") (OtherBodyIndex :type Integer) (bFromSweep :type Boolean) (SweepResult :type "HitResult Structure (by ref)"))
  (cast `/Game/BP_Bullet` OtherActor)
  (set `self.Life` (- (`self.Life`) 1.0))
  (`self.K2_DestroyActor` OtherActor))

(fn `UserConstructionScript`)