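; BP_GameManager runs the zombie wave loop and adds the HUD and game over screen.
; Tick counts down between waves, then spawns as many BP_Zombie as the wave number at random navigable points around the player and resets BP_AmmoCounter's bullets.
; It polls the remaining zombie count to restart the countdown when none are left.
; While BP_Player is dead, it creates a new WB_GameOver widget every frame.
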(event `self.ReceiveBeginPlay`
  (bind _returnvalue (`|CreateWidget` "/Game/widgets/WB_HUD.WB_HUD_C" (`GameplayStatics.GetPlayerController` 0)))
  (bind _output_get (set `self.HUD` _returnvalue))
  (`UserWidget.AddToViewport` _output_get 0)
  (set `self.WaveCD` 5.0))

(event `self.ReceiveTick`
  (params (DeltaSeconds :type "Float (single-precision)"))
  (bind _wave (`self.Wave`))
  (`|ExecutionSequence`
    (:`then_0`
      (if (not (`self.OnWave`))
        (set `self.WaveCD` (- (`self.WaveCD`) DeltaSeconds))))
    (:`then_1`
      (if (<= (`self.WaveCD`) 0.0)
        (set `self.OnWave` true)
        (`|ExecutionSequence`
          (:`then_0`
            (if (not (`self.MidWave`))
              (`/Engine/EditorBlueprintResources/StandardMacros.IncrementInt` _wave
                (:`  `
                  (set `self.SpawnsLeft` _wave)
                  (set `self.MidWave` true)
                  (bind _returnvalue (`GameplayStatics.GetActorOfClass` "/Game/BP_AmmoCounter.BP_AmmoCounter_C"))
                  (set `/Game/BP_AmmoCounter.Bullets` 2 _returnvalue)))))
          (:`then_1`
            (while (> (`self.SpawnsLeft`) 0)
              (`|SpawnActorFromClass` "/Game/BP_Zombie.BP_Zombie_C" (`KismetMathLibrary.MakeTransform` (`NavigationSystemV1.K2_GetRandomReachablePointInRadius` (`self.K2_GetActorLocation` (`GameplayStatics.GetPlayerPawn` 0)) 3000.0 null null)) "Undefined" "MultiplyWithRoot" null null)
              (`/Engine/EditorBlueprintResources/StandardMacros.DecrementInt` (`self.SpawnsLeft`)))
            (bind _outactors (`GameplayStatics.GetAllActorsOfClass` "/Game/BP_Zombie.BP_Zombie_C"))
            (set `self.TotalEnemies` (`KismetArrayLibrary.Array_Length` _outactors))
            (if (== (`self.TotalEnemies`) 0)
              (set `self.WaveCD` 5.0)
              (set `self.OnWave` false)
              (set `self.MidWave` false))))))
    (:`then_2`
      (bind _returnvalue_2 (`GameplayStatics.GetActorOfClass` "/Game/BP_Player.BP_Player_C"))
      (if (`/Game/BP_Player.IsDead` _returnvalue_2)
        (bind _returnvalue_3 (`|CreateWidget` "/Game/widgets/WB_GameOver.WB_GameOver_C" (`GameplayStatics.GetPlayerController` 0)))
        (`UserWidget.AddToViewport` _returnvalue_3 0)))))

(fn `UserConstructionScript`)