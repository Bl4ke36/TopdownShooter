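; BP_Zombie is a zombie enemy that walks straight at the player, attacks at close range and adds to the score when killed.
; Tick turns it toward the player and applies movement input without pathfinding, and at zero Life increments BP_GameManager's Score and destroys it.
; Overlapping Rango stops movement, sets AB_zombie's Attacking flag and starts a Delay-driven damage loop on whatever entered, until any actor overlap ends.
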(event `self.ReceiveTick`
  (params (DeltaSeconds :type "Float (single-precision)"))
  (bind (_returnvalue_roll _returnvalue_pitch _returnvalue_yaw) (`KismetMathLibrary.BreakRotator` (`KismetMathLibrary.FindLookAtRotation` (`self.K2_GetActorLocation` self) (`self.K2_GetActorLocation` (`GameplayStatics.GetPlayerPawn` 0)))))
  (`|ExecutionSequence`
    (:`then_0`
      (if (not (> (`self.Life`) 0.0))
        (bind _returnvalue (`GameplayStatics.GetActorOfClass` "/Game/BP_GameManager.BP_GameManager_C"))
        (`/Engine/EditorBlueprintResources/StandardMacros.IncrementInt` (`/Game/BP_GameManager.Score` _returnvalue)
          (:`  `
            (`self.K2_DestroyActor`)))))
    (:`then_1`
      (if (not (`self.OnRange`))
        (`/Engine/EditorBlueprintResources/StandardMacros.IsValid` self
          (:`Is Valid`
            (`self.K2_SetActorRotation` (`KismetMathLibrary.MakeRotator` 0.0 0.0 _returnvalue_yaw))
            (`self.AddMovementInput` (`self.GetActorForwardVector` self) 0.5)))))))

(event `self.ReceiveBeginPlay`
  (set `self.Life` 30.0))

(event `self.ReceiveAnyDamage`
  (params (Damage :type "Float (single-precision)") (DamageType :type "DamageType Object Reference") (InstigatedBy :type "Controller Object Reference") (DamageCauser :type "Actor Object Reference"))
  (set `self.Life` (- (`self.Life`) Damage)))

(event `self.Rango.OnComponentBeginOverlap`
  (params (OverlappedComponent :type "PrimitiveComponent Object Reference") (OtherActor :type "Actor Object Reference") (OtherComp :type "PrimitiveComponent Object Reference") (OtherBodyIndex :type Integer) (bFromSweep :type Boolean) (SweepResult :type "HitResult Structure (by ref)"))
  (bind _asab_zombie (cast `/Game/AB_zombie` (`SkeletalMeshComponent.GetAnimInstance` (`self.Mesh`))))
  (set `/Game/AB_zombie.Attacking` true _asab_zombie)
  (set `self.OnRange` true)
  (`KismetSystemLibrary.Delay` 1.0)
  (if (`self.OnRange`)
    (`GameplayStatics.ApplyDamage` OtherActor 10.0 null self :!label _label)
    (`KismetSystemLibrary.Delay` 2.6)
    (if (`self.OnRange`)
      (goto _label))))

(event `self.ReceiveActorEndOverlap`
  (params (OtherActor :type "Actor Object Reference"))
  (bind _asab_zombie (cast `/Game/AB_zombie` (`SkeletalMeshComponent.GetAnimInstance` (`self.Mesh`))))
  (set `/Game/AB_zombie.Attacking` false _asab_zombie)
  (set `self.OnRange` false))

(fn `UserConstructionScript`)